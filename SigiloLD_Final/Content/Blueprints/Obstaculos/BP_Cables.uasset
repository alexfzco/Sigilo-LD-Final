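; BP_Cables is a tripwire obstacle that hurts the player and makes a loud noise when crossed.
; At BeginPlay it stretches a thin cylinder between the Inicio and Final points, procedurally easing level design.
; Each tick a line trace between those points checks for BP_Player.
; The first hit subtracts health, plays a sound and reports an AI noise event at the midpoint, then destroys the actor after a delay.
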(event EventTick
  (params (DeltaSeconds :type Float%20%28single-precision%29))
  (bind _final (Variables|Default|GetFinal))
  (bind _inicio (Variables|Default|GetInicio))
  (bind _returnvalue (Transformation|GetWorldTransform _final))
  (bind _returnvalue_2 (Transformation|GetWorldTransform _inicio))
  (bind _returnvalue_3 (+ (.location _returnvalue_2) (.location _returnvalue)))
  (bind _returnvalue_4 (/ _returnvalue_3 2.0))
  ;[0.15 0.15 0.15 0.5] Logica de contacto
  (Variables|Default|SetDraw%20Debug%20Type "Persistent")
  (bind _outhit (Collision|LineTraceByChannel (.location _returnvalue_2) (.location _returnvalue) "TraceTypeQuery3" false 0 (Variables|Default|GetDraw%20Debug%20Type)))
  (bind _asbp_player (Utilities|Casting|CastToBP_Player (.HitActor (Collision|BreakHitResult _outhit))))
  (Utilities|FlowControl|DoOnce false
    (:Completed
      (Variables|Default|SetDraw%20Debug%20Type "None")
      (Variables|/Game/Blueprints/BP_Player.BP_Player_C|SetHealth _asbp_player (- (Variables|/Game/Blueprints/BP_Player.BP_Player_C|GetHealth _asbp_player) 5e+01))
      (Audio|PlaySoundatLocation "/Engine/EditorSounds/Notifications/CompileFailed.CompileFailed" _returnvalue_4 "0, 0, 0" 1.0 1.0 0.0 0 0 0 0)
      (Class|AISenseHearing|ReportNoiseEvent _returnvalue_4 99999.0 0 (Variables|Default|GetMax%20Range) "None")
      (Utilities|FlowControl|Delay 2.0)
      (Actor|DestroyActor))))

(event EventBeginPlay
  ;[0.15 0.15 0.15 0.5] Crear cilindro de forma procedural para facilitar el diseño de nivel
  (Transformation|SetWorldLocation (Variables|Default|GetCylinder) (|Palmedio_2) false false)
  (Transformation|SetWorldRotation (Variables|Default|GetCylinder) (|Rotao_2) false false)
  (Transformation|SetWorldScale3D (Variables|Default|GetCylinder) (|Escalao_2)))

(fn ConstructionScript)