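; BP_PulseGrenade is a thrown grenade that temporarily disables CCTV cameras.
; On BeginPlay it launches forward with an upward arc through ProjectileMovement, then detonates after a short delay.
; The pulse hides the mesh, enables the PulseRadius query volume and disables overlapping BP_CCTV_Cam actors.
; A timer set inside that loop later re-enables cameras still overlapping and destroys the grenade, so cleanup requires at least one camera caught.
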(event Custom|ExplodePulse
  (Rendering|SetVisibility (Variables|Default|GetPulseRadius) true false)
  (Collision|SetCollisionEnabled (Variables|Default|GetPulseRadius) "QueryOnly")
  (Rendering|SetVisibility (Variables|Default|GetGrenadeMesh) false false)
  (for _array_element (Collision|GetOverlappingActors (Variables|Default|GetPulseRadius) "/Game/LevelDesignKit/Blueprints/BP_CCTV_Cam.BP_CCTV_Cam_C" :!class /Script/Engine.PrimitiveComponent)
    (bind _asbp_cctv_cam (Utilities|Casting|CastToBP_CCTV_Cam _array_element))
    (Default|DisableCamera _asbp_cctv_cam)
    (Utilities|Time|SetTimerbyEvent (delegate Custom|ReactivarCamaras) 6.0)))

(event Custom|ReactivarCamaras
  (for _array_element (Collision|GetOverlappingActors (Variables|Default|GetPulseRadius) "/Game/LevelDesignKit/Blueprints/BP_CCTV_Cam.BP_CCTV_Cam_C" :!class /Script/Engine.PrimitiveComponent)
    (bind _asbp_cctv_cam (Utilities|Casting|CastToBP_CCTV_Cam _array_element))
    (Default|EnableCamera _asbp_cctv_cam))
  (Actor|DestroyActor))

(event EventBeginPlay
  (bind _pulseradius (Variables|Default|GetPulseRadius))
  (Rendering|SetVisibility _pulseradius false false)
  (Collision|SetCollisionEnabled _pulseradius "NoCollision")
  (Variables|/Script/Engine.MovementComponent|SetVelocity (Variables|Default|GetProjectileMovement) (+ (* (Transformation|GetActorForwardVector) "1500.000000,1500.000000,1500.000000") (Math|Vector|MakeVector 0.0 0.0 3e+02)))
  (Utilities|FlowControl|Delay 3.0)
  (CallFunction|ExplodePulse))

(fn ConstructionScript)