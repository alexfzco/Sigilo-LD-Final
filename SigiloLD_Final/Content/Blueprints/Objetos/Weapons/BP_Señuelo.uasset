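; BP_Señuelo is a thrown decoy that emits a noise AI hearing can detect.
; On BeginPlay it launches along its forward vector with an upward arc through ProjectileMovement, then waits briefly before triggering its sound event.
; That event plays a "pspsps" sound and reports a loud, long-range noise at its location, with itself as instigator, then destroys the actor after a short delay.
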(event Custom|CE_MakeSound
  (Audio|PlaySoundatLocation "/Game/Sounds/pspspspspsp-made-with-Voicemod__mp3cut_net_.pspspspspsp-made-with-Voicemod__mp3cut_net_" (Transformation|GetActorLocation) "0, 0, 0" 1.0 1.0 0.0 0 0 0 0)
  (Class|AISenseHearing|ReportNoiseEvent (Transformation|GetActorLocation) 2e+04 self 1e+05 "None")
  (Utilities|FlowControl|Delay 1.0)
  (Actor|DestroyActor))

(event EventBeginPlay
  (Variables|/Script/Engine.MovementComponent|SetVelocity (Variables|Default|GetProjectileMovement) (+ (* (Transformation|GetActorForwardVector) "1000.000000,1000.000000,1000.000000") (Math|Vector|MakeVector 0.0 0.0 3e+02)))
  (Utilities|FlowControl|Delay 2.0)
  (CallFunction|CEMakeSound))

(fn ConstructionScript)