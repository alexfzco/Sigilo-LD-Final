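; BP_SmokeGrenade is a thrown smoke grenade projectile that deploys a smoke cloud after a short fuse.
; BeginPlay hides and disables the ColliderHumo smoke collider, launches ProjectileMovement forward with an upward arc, then calls Explode after a delay.
; Explode shows the collider as query-only and spawns the Niagara smoke at the grenade's location.
; After the smoke duration it destroys the actor, then the Niagara component.
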(event Custom|Explode
  (bind _colliderhumo (Variables|Default|GetColliderHumo))
  ;[0.15 0.15 0.15 0.5] CE_Explode
  (Rendering|SetVisibility _colliderhumo true false)
  (Collision|SetCollisionEnabled _colliderhumo "QueryOnly")
  (bind _returnvalue (Niagara|SpawnSystematLocation "/Game/LevelDesignKit/VFX/NS_Smoke02.NS_Smoke02" (Transformation|GetActorLocation)))
  (Utilities|FlowControl|Delay 1e+01)
  (Actor|DestroyActor)
  (Components|DestroyComponent _returnvalue))

(event EventBeginPlay
  (bind _colliderhumo (Variables|Default|GetColliderHumo))
  ;[0.15 0.15 0.15 0.5] BeginPlay
  (Rendering|SetVisibility _colliderhumo false false)
  (Collision|SetCollisionEnabled _colliderhumo "NoCollision")
  (Variables|/Script/Engine.MovementComponent|SetVelocity (Variables|Default|GetProjectileMovement) (+ (* (Transformation|GetActorForwardVector) "1500.000000,1500.000000,1500.000000") (Math|Vector|MakeVector 0.0 0.0 3e+02)))
  (Utilities|FlowControl|Delay 3.0)
  (CallFunction|Explode))

(fn ConstructionScript)