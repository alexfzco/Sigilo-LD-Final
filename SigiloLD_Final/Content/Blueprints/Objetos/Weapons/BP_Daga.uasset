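; BP_Daga is a dagger weapon projectile that homes in on one target enemy and kills it instantly.
; On BeginPlay, if TargetEnemy is valid, it enables homing on ProjectileMovement and sets the enemy's Mesh as the homing target.
; When its Sphere overlaps that enemy, it calls InstantKill on it and destroys itself, ignoring every other actor.
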(event OnComponentBeginOverlap(Sphere)
  (params (OverlappedComponent :type Primitive%20Component%20Object%20Reference) (OtherActor :type Actor%20Object%20Reference) (OtherComp :type Primitive%20Component%20Object%20Reference) (OtherBodyIndex :type Integer) (bFromSweep :type Boolean) (SweepResult :type Hit%20Result%20Structure%20%28by%20ref%29))
  (if (== OtherActor (Variables|Default|GetTargetEnemy))
    (Default|InstantKill (Variables|Default|GetTargetEnemy))
    (Actor|DestroyActor)))

(event EventBeginPlay
  (Utilities|IsValid (Variables|Default|GetTargetEnemy)
    (:Is%20Valid
      (Variables|/Script/Engine.ProjectileMovementComponent|SetbIsHomingProjectile (Variables|Default|GetProjectileMovement) true)
      (Variables|/Script/Engine.ProjectileMovementComponent|SetHomingTargetComponent (Variables|Default|GetProjectileMovement) (Variables|/Script/Engine.Character|GetMesh (Variables|Default|GetTargetEnemy))))))

(fn ConstructionScript)