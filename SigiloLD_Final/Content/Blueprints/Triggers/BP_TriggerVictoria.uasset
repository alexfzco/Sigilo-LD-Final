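; BP_TriggerVictoria is a victory trigger that shows a win screen when BP_Player overlaps its Box.
; The overlap pauses the game before casting, so it stays paused for any other actor.
; For the player, it adds WBP_VictoriaBueno, zeroes walk speed and unpauses.
; After a five-second delay it opens the Blockout level, then removes the widget and restores walk speed.
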(event OnComponentBeginOverlap(Box)
  (params (OverlappedComponent :type Primitive%20Component%20Object%20Reference) (OtherActor :type Actor%20Object%20Reference) (OtherComp :type Primitive%20Component%20Object%20Reference) (OtherBodyIndex :type Integer) (bFromSweep :type Boolean) (SweepResult :type Hit%20Result%20Structure%20%28by%20ref%29))
  (Game|SetGamePaused true)
  (bind _asbp_player (Utilities|Casting|CastToBP_Player OtherActor))
  (bind _returnvalue (UserInterface|CreateWidget "/Game/Blueprints/Widgets/WBP_VictoriaBueno.WBP_VictoriaBueno_C"))
  (UserInterface|Viewport|AddtoViewport _returnvalue 0)
  (Variables|/Script/Engine.CharacterMovementComponent|SetMaxWalkSpeed (Variables|/Script/Engine.Character|GetCharacterMovement _asbp_player) 0.0)
  (Game|SetGamePaused false)
  (Utilities|FlowControl|Delay 5.0)
  (Game|OpenLevel(byObjectReference) "/Game/Levels/Blockout.Blockout")
  (Widget|RemovefromParent _returnvalue)
  (Variables|/Script/Engine.CharacterMovementComponent|SetMaxWalkSpeed (Variables|/Script/Engine.Character|GetCharacterMovement _asbp_player) 6e+02))

(event EventBeginPlay)

(event Collision|EventActorBeginOverlap
  (params (OtherActor :type Actor%20Object%20Reference)))

(event EventTick
  (params (DeltaSeconds :type Float%20%28single-precision%29)))

(fn ConstructionScript)