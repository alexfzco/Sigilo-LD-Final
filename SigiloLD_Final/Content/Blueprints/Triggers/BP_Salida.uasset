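; BP_Salida is an exit ("salida") actor that shows a notice near it and removes itself once no enemies remain in the level.
; On BeginPlay it adds a Wbp_avisoInstrucciones widget with hidden text, which the TriggerTexto overlap shows and hides without filtering the overlapping actor.
; A looping timer polls GetAllActorsOfClass for BP_Enemy_Base and destroys the actor when the result is empty.
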(event OnComponentBeginOverlap(triggerTexto)
  (params (OverlappedComponent :type Primitive%20Component%20Object%20Reference) (OtherActor :type Actor%20Object%20Reference) (OtherComp :type Primitive%20Component%20Object%20Reference) (OtherBodyIndex :type Integer) (bFromSweep :type Boolean) (SweepResult :type Hit%20Result%20Structure%20%28by%20ref%29))
  (Widget|SetVisibility (Variables|/Game/Blueprints/wbp_avisoInstrucciones.wbp_avisoInstrucciones_C|GetTextoAviso (Variables|Default|GetWidgetSalida)) "Visible"))

(event OnComponentEndOverlap(triggerTexto)
  (params (OverlappedComponent :type Primitive%20Component%20Object%20Reference) (OtherActor :type Actor%20Object%20Reference) (OtherComp :type Primitive%20Component%20Object%20Reference) (OtherBodyIndex :type Integer))
  (Widget|SetVisibility (Variables|/Game/Blueprints/wbp_avisoInstrucciones.wbp_avisoInstrucciones_C|GetTextoAviso (Variables|Default|GetWidgetSalida)) "Hidden"))

(event Custom|CE_ComprobarEnemigos
  (bind _outactors (Actor|GetAllActorsOfClass "/Game/Blueprints/Characters/Enemies/BP_Enemy_Base.BP_Enemy_Base_C"))
  (if (== (Utilities|Array|Length _outactors) 0)
    (Actor|DestroyActor)))

(event EventBeginPlay
  (bind _returnvalue (UserInterface|CreateWidget "/Game/Blueprints/wbp_avisoInstrucciones.wbp_avisoInstrucciones_C"))
  (bind _output_get (Variables|Default|SetWidgetSalida _returnvalue))
  (Widget|SetVisibility (Variables|/Game/Blueprints/wbp_avisoInstrucciones.wbp_avisoInstrucciones_C|GetTextoAviso _output_get) "Hidden")
  (UserInterface|Viewport|AddtoViewport _output_get 0)
  (Utilities|Time|SetTimerbyEvent (delegate Custom|CE_ComprobarEnemigos) 1.0 true))

(fn ConstructionScript)