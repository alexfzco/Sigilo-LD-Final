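; BP_SmokeGrenade is a thrown smoke grenade actor that deploys a timed smoke cloud.
; On BeginPlay it hides and disables its smoke collider, launches forward with an upward arc through ProjectileMovement, and waits a short fuse.
; Explode then shows the collider as query-only, spawns a Niagara smoke effect at the grenade's location, and destroys the actor after a delay.
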(event Custom|Explode
  (bind _colliderhumo (Variables|Default|GetColliderHumo))
  (Rendering|SetVisibility _colliderhumo true false)
  (Collision|SetCollisionEnabled _colliderhumo "QueryOnly")
  (Niagara|SpawnSystematLocation "/Game/LevelDesignKit/VFX/NS_Smoke02.NS_Smoke02" (Transformation|GetActorLocation))
  (Utilities|FlowControl|Delay 1e+01)
  (Actor|DestroyActor))

(event EventBeginPlay
  (bind _colliderhumo (Variables|Default|GetColliderHumo))
  (Rendering|SetVisibility _colliderhumo false false)
  (Collision|SetCollisionEnabled _colliderhumo "NoCollision")
  (Variables|/Script/Engine.MovementComponent|SetVelocity (Variables|Default|GetProjectileMovement) (+ (* (Transformation|GetActorForwardVector) "1500.000000,1500.000000,1500.000000") (Math|Vector|MakeVector 0.0 0.0 3e+02)))
  (Utilities|FlowControl|Delay 2.0)
  (CallFunction|Explode))

(fn ConstructionScript)