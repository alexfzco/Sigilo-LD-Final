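; Base enemy character with health, a melee-style attack, target highlighting and helper functions for patrol route and movement speed.
; The attack damages the player immediately, without a range check, then plays a montage and signals attack end on completion or interruption.
; Incoming damage reduces and prints health, destroying the actor at zero or on instant kill.
; Marking swaps the mesh material to red, and unmarking restores the original cached at BeginPlay.
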(event Custom|MarcarObjetivo
  (Rendering|Material|SetMaterial (Variables|Character|GetMesh) 0 (Variables|Default|GetMaterialRojo)))

(event Custom|CE_Attack
  ;[0.15 0.15 0.15 0.5] Attack
  (Game|Damage|ApplyDamage (Game|GetPlayerCharacter 0) (Variables|Default|GetBase%20Damage) 0 0 "/Script/Engine.DamageType")
  (Animation|Montage|PlayMontage (Variables|Character|GetMesh) "/Game/Materials/Mannequins/Anims/Unarmed/Attack/MM_Attack_01_Montage.MM_Attack_01_Montage"
    (:OnCompleted
      _)
    (:OnInterrupted
      _))
  (Default|CallOnAttackEnd))

(event Custom|DesmarcarObjetivo
  (Rendering|Material|SetMaterial (Variables|Character|GetMesh) 0 (Variables|Default|GetMaterialOriginal)))

(event Custom|InstantKill
  (Actor|DestroyActor))

(event EventBeginPlay
  (Variables|Default|SetMaterialOriginal (Rendering|Material|GetMaterial (Variables|Character|GetMesh) 0))
  ;[0.15 0.15 0.15 0.5] Vida
  (Variables|Default|SetHealth (Variables|Default|GetMaxHealth)))

(event Game|Damage|EventAnyDamage
  (params (Damage :type Float%20%28single-precision%29) (DamageType :type Damage%20Type%20Object%20Reference) (InstigatedBy :type Controller%20Object%20Reference) (DamageCauser :type Actor%20Object%20Reference))
  ;[0.15 0.15 0.15 0.5] AnyDamage
  (bind _output_get (Variables|Default|SetHealth (- (Variables|Default|GetHealth) Damage)))
  (Development|PrintString (Utilities|String|ToString(Float) _output_get))
  (if (<= _output_get 0.0)
    (Actor|DestroyActor)))

(fn ConstructionScript)

(fn GetPatrolRoute
  (return (Variables|AI|GetPatrolRoute)))

(fn SetMovementSpeed
  (params (Speed :type E_MovementSpeed%20Enum :default "NewEnumerator0"))
  (Variables|/Script/Engine.CharacterMovementComponent|SetMaxWalkSpeed (Variables|Character|GetCharacterMovement) (Utilities|Select :Index Speed :NewEnumerator0 0.0 :NewEnumerator1 2e+02 :NewEnumerator2 4e+02 :NewEnumerator3 6e+02))
  (return 0.0))