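; BP_CCTV_Cam is a security camera that sweeps via a timeline, unless Stationary, and detects the player with a vision-cone trigger.
; Detection reports a noise event and, while powered, halts rotation, turns the cone red and sounds an alarm.
; Leaving triggers a delayed yellow suspicion phase before normal operation resumes.
; A hit, or pressing E at the optional power button, shuts the camera off and hides its cone.
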(event OnComponentBeginOverlap(TV_Press)
  (params (OverlappedComponent :type Primitive%20Component%20Object%20Reference) (OtherActor :type Actor%20Object%20Reference) (OtherComp :type Primitive%20Component%20Object%20Reference) (OtherBodyIndex :type Integer) (bFromSweep :type Boolean) (SweepResult :type Hit%20Result%20Structure%20%28by%20ref%29))
  ;[1 1 1] Check If Player is CLose to Button
  (if (Variables|CCTV_Inputs|GetPower_Button)
    (Input|EnableInput (Game|GetPlayerController 0))))

(event OnComponentEndOverlap(TV_Press)
  (params (OverlappedComponent :type Primitive%20Component%20Object%20Reference) (OtherActor :type Actor%20Object%20Reference) (OtherComp :type Primitive%20Component%20Object%20Reference) (OtherBodyIndex :type Integer))
  ;[1 1 1] Check If Player is CLose to Button
  (if (Variables|CCTV_Inputs|GetPower_Button)
    (Input|DisableInput (Game|GetPlayerController 0))))

(event OnComponentBeginOverlap(TV_Spotted)
  (params (OverlappedComponent :type Primitive%20Component%20Object%20Reference) (OtherActor :type Actor%20Object%20Reference) (OtherComp :type Primitive%20Component%20Object%20Reference) (OtherBodyIndex :type Integer) (bFromSweep :type Boolean) (SweepResult :type Hit%20Result%20Structure%20%28by%20ref%29))
  ;[1 1 1] Player Triggers Alarm
  (Utilities|Casting|CastToBP_Player OtherActor)
  (if true
    (Class|AISenseHearing|ReportNoiseEvent (Variables|Default|GetLocation) 2e+03 self 1e+03 "None")
    (if (Variables|CCTV_Inputs|GetPowerOn)
      (Utilities|FlowControl|Sequence
        (:then_0
          ;[1 1 1] Camera Rotation
          (bind _rotation (Timeline|Rotation Stop)
            (:Update
              (Transformation|SetRelativeRotation (Variables|Default|GetSM_SecurityCamera) (Math|Rotator|MakeRotator 0.0 0.0 (* _rotation (Variables|CCTV_Inputs|GetCamera_Rotation_Angle))) false false))))
        (:then_1
          (Rendering|SetVisibility (Variables|Default|GetSM_ExclamationPoint) true false)
          (Rendering|Material|SetMaterial (Variables|Default|GetCone) 0 "/Game/LevelDesignKit/Material/MI_BulletProofGlass_Red.MI_BulletProofGlass_Red")
          (Audio|Components|Audio|Play (Variables|Default|GetSFX_ButtonPressed_On) 0.0))))))

(event OnComponentEndOverlap(TV_Spotted)
  (params (OverlappedComponent :type Primitive%20Component%20Object%20Reference) (OtherActor :type Actor%20Object%20Reference) (OtherComp :type Primitive%20Component%20Object%20Reference) (OtherBodyIndex :type Integer))
  ;[1 1 1] When players leave Camera FoV
  (Utilities|Casting|CastToBP_Player OtherActor)
  (if true
    (if (Variables|CCTV_Inputs|GetPowerOn)
      (Utilities|FlowControl|Delay 1.5)
      (Rendering|SetVisibility (Variables|Default|GetSM_ExclamationPoint) false false)
      (Rendering|SetVisibility (Variables|Default|GetSM_InterrogationPoint) true false)
      (Rendering|Material|SetMaterial (Variables|Default|GetCone) 0 "/Game/LevelDesignKit/Material/MI_BulletProofGlass_Yellow.MI_BulletProofGlass_Yellow")
      (Utilities|FlowControl|Delay 3.0)
      (Rendering|SetVisibility (Variables|Default|GetSM_InterrogationPoint) false false)
      (Rendering|Material|SetMaterial (Variables|Default|GetCone) 0 "/Game/LevelDesignKit/Material/MI_BulletProofGlass.MI_BulletProofGlass")
      (Utilities|FlowControl|Sequence
        (:then_0
          (if (Variables|CCTV_Inputs|GetPowerOn)
            (if (not (Variables|CCTV_Inputs|GetStationary))
              ;[1 1 1] Camera Rotation
              (bind _rotation (Timeline|Rotation Play)
                (:Update
                  (Transformation|SetRelativeRotation (Variables|Default|GetSM_SecurityCamera) (Math|Rotator|MakeRotator 0.0 0.0 (* _rotation (Variables|CCTV_Inputs|GetCamera_Rotation_Angle))) false false))))))
        (:then_1
          (Audio|Components|Audio|Stop (Variables|Default|GetSFX_ButtonPressed_On)))))))

(event EventBeginPlay
  ;[1 1 1] Start set ! Invisible and start roataion
  (Variables|CCTV_Inputs|SetPowerOn true)
  (Rendering|SetVisibility (Variables|Default|GetSM_InterrogationPoint) false false)
  (Rendering|SetVisibility (Variables|Default|GetSM_ExclamationPoint) false false)
  (if (not (Variables|CCTV_Inputs|GetStationary))
    ;[1 1 1] Camera Rotation
    (bind _rotation (Timeline|Rotation Play)
      (:Update
        (Transformation|SetRelativeRotation (Variables|Default|GetSM_SecurityCamera) (Math|Rotator|MakeRotator 0.0 0.0 (* _rotation (Variables|CCTV_Inputs|GetCamera_Rotation_Angle))) false false)))))

(event Collision|EventHit
  (params (MyComp :type Primitive%20Component%20Object%20Reference) (Other :type Actor%20Object%20Reference) (OtherComp :type Primitive%20Component%20Object%20Reference) (bSelfMoved :type Boolean) (HitLocation :type Vector :default "0, 0, 0") (HitNormal :type Vector :default "0, 0, 0") (NormalImpulse :type Vector :default "0, 0, 0") (Hit :type Hit%20Result%20Structure%20%28by%20ref%29))
  ;[1 1 1] Turn off Power to CCTV Cam
  (if (Variables|CCTV_Inputs|GetStationary)
    (Variables|CCTV_Inputs|SetPowerOn false :!label _label)
    (Rendering|Material|SetMaterial (Variables|Default|GetSM_Button) 0 "/Game/LevelDesignKit/Material/MI_Color_Green.MI_Color_Green")
    (Audio|PlaySound2D "/Game/LevelDesignKit/Audio/SFX_ButtonPressed_On.SFX_ButtonPressed_On" 1.0 1.0 0.0 0 0)
    (Rendering|Material|SetMaterial (Variables|Default|GetSM_SecurityCamera) 0 "/Game/LevelDesignKit/Material/Master/M_ColorNoShadow.M_ColorNoShadow")
    (Rendering|SetVisibility (Variables|Default|GetCone) false false)
    (else
      (Utilities|FlowControl|Sequence
        (:then_0
          ;[1 1 1] Camera Rotation
          (bind _rotation (Timeline|Rotation Stop)
            (:Update
              (Transformation|SetRelativeRotation (Variables|Default|GetSM_SecurityCamera) (Math|Rotator|MakeRotator 0.0 0.0 (* _rotation (Variables|CCTV_Inputs|GetCamera_Rotation_Angle))) false false))))
        (:then_1
          (goto _label))))))

(event Input|KeyboardEvents|E
  (params (Key :type Key%20Structure :default "None"))
  ;[1 1 1] Turn off Power to CCTV Cam
  (:Pressed
    (if (Variables|CCTV_Inputs|GetPower_Button)
      (if (Variables|CCTV_Inputs|GetStationary)
        (Variables|CCTV_Inputs|SetPowerOn false :!label _label)
        (Rendering|Material|SetMaterial (Variables|Default|GetSM_Button) 0 "/Game/LevelDesignKit/Material/MI_Color_Green.MI_Color_Green")
        (Audio|PlaySound2D "/Game/LevelDesignKit/Audio/SFX_ButtonPressed_On.SFX_ButtonPressed_On" 1.0 1.0 0.0 0 0)
        (Rendering|Material|SetMaterial (Variables|Default|GetSM_SecurityCamera) 0 "/Game/LevelDesignKit/Material/Master/M_ColorNoShadow.M_ColorNoShadow")
        (Rendering|SetVisibility (Variables|Default|GetCone) false false)
        (else
          (Utilities|FlowControl|Sequence
            (:then_0
              ;[1 1 1] Camera Rotation
              (bind _rotation (Timeline|Rotation Stop)
                (:Update
                  (Transformation|SetRelativeRotation (Variables|Default|GetSM_SecurityCamera) (Math|Rotator|MakeRotator 0.0 0.0 (* _rotation (Variables|CCTV_Inputs|GetCamera_Rotation_Angle))) false false))))
            (:then_1
              (goto _label))))))))

(fn ConstructionScript
  (if (Variables|CCTV_Inputs|GetPower_Button)
    (|ShowButton)
    (else
      (|HideButton))))

(fn DisableCamera
  (Actor|Tick|SetActorTickEnabled false)
  (Variables|CCTV_Inputs|SetPowerOn false)
  (Rendering|SetVisibility (Variables|Default|GetCone) false false))

(fn EnableCamera
  (Variables|CCTV_Inputs|SetPowerOn true)
  (Actor|Tick|SetActorTickEnabled true)
  (Rendering|SetVisibility (Variables|Default|GetCone) false false))